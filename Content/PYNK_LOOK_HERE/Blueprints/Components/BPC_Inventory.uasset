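; Inventory component that stores item stacks in a bag array and in equipment slots for head, body, weapon, explosive and two tarots.
; AddToInventory fills a given slot or auto-places items by matching stackable name, falling back to the first empty index.
; RemoveFromInventory clears slots or reduces quantities, though its bag clamp zeroes any partial removal.
; IsFull checks only the bag for stackable matches or empty slots, leaving its equipment check disconnected.
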(fn AddtoInventory
  (params (Item :type F%20Item%20Details%20Structure) (Equipped :type Boolean) (SlotIndex :type Integer) (EquipmentSlot :type E_ItemType%20Enum :default "NewEnumerator0"))
  (LocalVariables|SetItemDetails Item)
  (LocalVariables|SetIndex SlotIndex)
  (LocalVariables|SetType EquipmentSlot)
  (if (< (.Quantity (Utilities|Struct|BreakF_ItemDetails (LocalVariables|GetItemDetails))) 1)
    (LocalVariables|SetItemDetails (Utilities|Struct|MakeF_ItemDetails (.Name (Utilities|Struct|BreakF_ItemDetails (LocalVariables|GetItemDetails))) (.Mesh (Utilities|Struct|BreakF_ItemDetails (LocalVariables|GetItemDetails))) (.Texture (Utilities|Struct|BreakF_ItemDetails (LocalVariables|GetItemDetails))) (.ItemType (Utilities|Struct|BreakF_ItemDetails (LocalVariables|GetItemDetails))) 1 (.Stackable (Utilities|Struct|BreakF_ItemDetails (LocalVariables|GetItemDetails))))))
  (if Equipped
    ;[1 1 1] Equip thing
    (switch Utilities|FlowControl|Switch|SwitchonE_ItemType (LocalVariables|GetType)
      (:NewEnumerator0
        (Variables|Equipped|SetHeadSlot (Utilities|Struct|MakeF_InventorySlot (LocalVariables|GetItemDetails) (.locked (Variables|Equipped|GetHeadSlot)))))
      (:NewEnumerator1
        (Variables|Equipped|SetBodySlot (Utilities|Struct|MakeF_InventorySlot (LocalVariables|GetItemDetails) (.locked (Variables|Equipped|GetBodySlot)))))
      (:NewEnumerator2
        (Variables|Equipped|SetWeaponSlot (Utilities|Struct|MakeF_InventorySlot (LocalVariables|GetItemDetails) (.locked (Variables|Equipped|GetWeaponSlot)))))
      (:NewEnumerator3
        (Variables|Equipped|SetExplosiveSlot (Utilities|Struct|MakeF_InventorySlot (Utilities|Struct|MakeF_ItemDetails (.name (LocalVariables|GetItemDetails)) (.mesh (LocalVariables|GetItemDetails)) (.texture (LocalVariables|GetItemDetails)) (.itemtype (LocalVariables|GetItemDetails)) (+ (.quantity (LocalVariables|GetItemDetails)) (.quantity (.itemdetails (Variables|Equipped|GetExplosiveSlot)))) true) (.stackable (LocalVariables|GetItemDetails)))))
      (:NewEnumerator4
        (switch int (LocalVariables|GetIndex)
          (:0
            (Variables|Equipped|SetTarotSlot1 (Utilities|Struct|MakeF_InventorySlot (LocalVariables|GetItemDetails) (.locked (Variables|Equipped|GetTarotSlot1)))))
          (:1
            (Variables|Equipped|SetTarotSlot2 (Utilities|Struct|MakeF_InventorySlot (LocalVariables|GetItemDetails) (.locked (Variables|Equipped|GetTarotSlot2))))))))
    (elif (== (LocalVariables|GetIndex) -1)
      ;[1 1 1] Looks scary, dont worry - all this does is loop through and stacks the new item if it can, if it can't it will find the first free slot and put it in there
      (LocalVariables|SetFirstEmptyIndex -1)
      (bind (_array_element _array_index) (Utilities|Array|ForEachLoopwithBreak (Variables|Default|GetInventory))
        (:LoopBody
          (LocalVariables|SetLoopIndex _array_index)
          (LocalVariables|SetCurrentQuantity (.quantity (.itemdetails _array_element)))
          ;;[1 1 1] Check if we can stack
          (if (and (Utilities|Enum|Equal(Enum) (.name (.itemdetails _array_element)) (.name (LocalVariables|GetItemDetails))) (.stackable (LocalVariables|GetItemDetails)))
            ;;[1 1 1] Add to existing
            (Utilities|Array|SetArrayElem (Variables|Default|GetInventory) (LocalVariables|GetLoopIndex) (Utilities|Struct|MakeF_InventorySlot (Utilities|Struct|MakeF_ItemDetails (.name (LocalVariables|GetItemDetails)) (.mesh (LocalVariables|GetItemDetails)) (.texture (LocalVariables|GetItemDetails)) (.itemtype (LocalVariables|GetItemDetails)) (+ (.quantity (LocalVariables|GetItemDetails)) (LocalVariables|GetCurrentQuantity)) (.stackable (LocalVariables|GetItemDetails))) false))
            (return)
            (else
              ;;[1 1 1] Make note of first found free slot
              (if (and (== (LocalVariables|GetCurrentQuantity) 0) (== (LocalVariables|GetFirstEmptyIndex) -1))
                (LocalVariables|SetFirstEmptyIndex (LocalVariables|GetLoopIndex))))))
        (:Completed
          ;;[1 1 1] Put in first free slot
          (Utilities|Array|SetArrayElem (Variables|Default|GetInventory) (LocalVariables|GetFirstEmptyIndex) (Utilities|Struct|MakeF_InventorySlot (LocalVariables|GetItemDetails) false))))
      (else
        ;;[1 1 1] Add thing to a specific slot in bag, stacking if applicable
        (if (== (.quantity (.itemdetails (Utilities|Array|Get(acopy) (Variables|Default|GetInventory) (LocalVariables|GetIndex)))) 0)
          (Utilities|Array|SetArrayElem (Variables|Default|GetInventory) (LocalVariables|GetIndex) (Utilities|Struct|MakeF_InventorySlot (LocalVariables|GetItemDetails) false))
          (else
            (Utilities|Array|SetArrayElem (Variables|Default|GetInventory) (LocalVariables|GetIndex) (Utilities|Struct|MakeF_InventorySlot (Utilities|Struct|MakeF_ItemDetails (.name (.itemdetails (Utilities|Array|Get(acopy) (Variables|Default|GetInventory) (LocalVariables|GetIndex)))) (.mesh (.itemdetails (Utilities|Array|Get(acopy) (Variables|Default|GetInventory) (LocalVariables|GetIndex)))) (.texture (.itemdetails (Utilities|Array|Get(acopy) (Variables|Default|GetInventory) (LocalVariables|GetIndex)))) (.itemtype (.itemdetails (Utilities|Array|Get(acopy) (Variables|Default|GetInventory) (LocalVariables|GetIndex)))) (+ (.quantity (.itemdetails (Utilities|Array|Get(acopy) (Variables|Default|GetInventory) (LocalVariables|GetIndex)))) (.quantity (LocalVariables|GetItemDetails))) (.stackable (.itemdetails (Utilities|Array|Get(acopy) (Variables|Default|GetInventory) (LocalVariables|GetIndex))))) false))))))))

(fn IsFull
  (params (ConsideredItemType :type E_ItemType%20Enum :default "NewEnumerator0") (ConsideredName :type String))
  (LocalVariables|SetType ConsideredItemType)
  (LocalVariables|SetName ConsideredName)
  ;[1 1 1] First check if any of the wildcards are empty
  (bind _array_element (Utilities|Array|ForEachLoopwithBreak (Variables|Default|GetInventory))
    (:LoopBody
      (if (or (and (Utilities|Enum|Equal(Enum) (.name (.itemdetails _array_element)) (LocalVariables|GetName)) (.stackable (.itemdetails _array_element))) (== (.quantity (.itemdetails _array_element)) 0))
        (return false)))
    (:Completed
      (return true))))

(fn RemovefromInventory
  (params (EquppedItem :type Boolean) (SlotIndex :type Integer) (EquipmentSlot :type E_ItemType%20Enum :default "NewEnumerator0") (Amount :type Integer))
  (bind _inventory (Variables|Default|GetInventory))
  (LocalVariables|SetIndex SlotIndex)
  (LocalVariables|SetReductionAmount Amount)
  (if EquppedItem
    (switch Utilities|FlowControl|Switch|SwitchonE_ItemType EquipmentSlot
      (:NewEnumerator0
        ;[1 1 1] Yeet
        (Variables|Equipped|SetHeadSlot (Utilities|Struct|MakeF_InventorySlot "(Name_6_D6936A53428A34342C39B89B41DE2056=\"\",Mesh_7_92FCB8BD4A0A9C4074E9D0A7872491F6=None,Texture_8_16B0979C40010D69A5EE2095A85FB3B7=None,ItemType_11_36FB1EB94DC6C6FF7EFC70984525A349=NewEnumerator0,Quantity_16_7F492F4B48DE614750C1C08C68CFB086=0,Stackable_18_364E31EB4817547950E5D6AA9CFEFB6F=True)" false)))
      (:NewEnumerator1
        (Variables|Equipped|SetBodySlot (Utilities|Struct|MakeF_InventorySlot "(Name_6_D6936A53428A34342C39B89B41DE2056=\"\",Mesh_7_92FCB8BD4A0A9C4074E9D0A7872491F6=None,Texture_8_16B0979C40010D69A5EE2095A85FB3B7=None,ItemType_11_36FB1EB94DC6C6FF7EFC70984525A349=NewEnumerator0,Quantity_16_7F492F4B48DE614750C1C08C68CFB086=0,Stackable_18_364E31EB4817547950E5D6AA9CFEFB6F=True)" false)))
      (:NewEnumerator2
        (Variables|Equipped|SetWeaponSlot (Utilities|Struct|MakeF_InventorySlot "(Name_6_D6936A53428A34342C39B89B41DE2056=\"\",Mesh_7_92FCB8BD4A0A9C4074E9D0A7872491F6=None,Texture_8_16B0979C40010D69A5EE2095A85FB3B7=None,ItemType_11_36FB1EB94DC6C6FF7EFC70984525A349=NewEnumerator0,Quantity_16_7F492F4B48DE614750C1C08C68CFB086=0,Stackable_18_364E31EB4817547950E5D6AA9CFEFB6F=True)" false)))
      (:NewEnumerator3
        ;[1 1 1] Check if we're removing all the explosives or just some
        (if (< (LocalVariables|GetReductionAmount) 1)
          (Variables|Equipped|SetExplosiveSlot (Utilities|Struct|MakeF_InventorySlot "(Name_6_D6936A53428A34342C39B89B41DE2056=\"\",Mesh_7_92FCB8BD4A0A9C4074E9D0A7872491F6=None,Texture_8_16B0979C40010D69A5EE2095A85FB3B7=None,ItemType_11_36FB1EB94DC6C6FF7EFC70984525A349=NewEnumerator0,Quantity_16_7F492F4B48DE614750C1C08C68CFB086=0,Stackable_18_364E31EB4817547950E5D6AA9CFEFB6F=True)" false))
          (else
            (Variables|Equipped|SetExplosiveSlot (Utilities|Struct|MakeF_InventorySlot (Utilities|Struct|MakeF_ItemDetails (.name (.itemdetails (Variables|Equipped|GetExplosiveSlot))) (.mesh (.itemdetails (Variables|Equipped|GetExplosiveSlot))) (.texture (.itemdetails (Variables|Equipped|GetExplosiveSlot))) (.itemtype (.itemdetails (Variables|Equipped|GetExplosiveSlot))) (- (.quantity (.itemdetails (Variables|Equipped|GetExplosiveSlot))) (LocalVariables|GetReductionAmount)) (.stackable (.itemdetails (Variables|Equipped|GetExplosiveSlot)))) (.locked (Variables|Equipped|GetExplosiveSlot)))))))
      (:NewEnumerator4
        ;[1 1 1] Remove tarot
        (switch int (LocalVariables|GetIndex)
          (:0
            (Variables|Equipped|SetTarotSlot1 (Utilities|Struct|MakeF_InventorySlot "(Name_6_D6936A53428A34342C39B89B41DE2056=\"\",Mesh_7_92FCB8BD4A0A9C4074E9D0A7872491F6=None,Texture_8_16B0979C40010D69A5EE2095A85FB3B7=None,ItemType_11_36FB1EB94DC6C6FF7EFC70984525A349=NewEnumerator0,Quantity_16_7F492F4B48DE614750C1C08C68CFB086=0,Stackable_18_364E31EB4817547950E5D6AA9CFEFB6F=True)" false)))
          (:1
            (Variables|Equipped|SetTarotSlot2 (Utilities|Struct|MakeF_InventorySlot "(Name_6_D6936A53428A34342C39B89B41DE2056=\"\",Mesh_7_92FCB8BD4A0A9C4074E9D0A7872491F6=None,Texture_8_16B0979C40010D69A5EE2095A85FB3B7=None,ItemType_11_36FB1EB94DC6C6FF7EFC70984525A349=NewEnumerator0,Quantity_16_7F492F4B48DE614750C1C08C68CFB086=0,Stackable_18_364E31EB4817547950E5D6AA9CFEFB6F=True)" false))))))
    (else
      ;[1 1 1] Remove thing from bag
      (if (< (LocalVariables|GetReductionAmount) 1)
        (Utilities|Array|SetArrayElem (Variables|Default|GetInventory) (LocalVariables|GetIndex) (Utilities|Struct|MakeF_InventorySlot "(Name_6_D6936A53428A34342C39B89B41DE2056=\"\",Mesh_7_92FCB8BD4A0A9C4074E9D0A7872491F6=None,Texture_8_16B0979C40010D69A5EE2095A85FB3B7=None,ItemType_11_36FB1EB94DC6C6FF7EFC70984525A349=NewEnumerator0,Quantity_16_7F492F4B48DE614750C1C08C68CFB086=0,Stackable_18_364E31EB4817547950E5D6AA9CFEFB6F=True)" false))
        (else
          (Utilities|Array|SetArrayElem _inventory (LocalVariables|GetIndex) (Utilities|Struct|MakeF_InventorySlot (Utilities|Struct|MakeF_ItemDetails (.name (.itemdetails (Utilities|Array|Get(acopy) _inventory (LocalVariables|GetIndex)))) (.mesh (.itemdetails (Utilities|Array|Get(acopy) _inventory (LocalVariables|GetIndex)))) (.texture (.itemdetails (Utilities|Array|Get(acopy) _inventory (LocalVariables|GetIndex)))) (.itemtype (.itemdetails (Utilities|Array|Get(acopy) _inventory (LocalVariables|GetIndex)))) (Math|Integer|Clamp(Integer) (- (.quantity (.itemdetails (Utilities|Array|Get(acopy) _inventory (LocalVariables|GetIndex)))) (LocalVariables|GetReductionAmount)) 0 0) (.stackable (.itemdetails (Utilities|Array|Get(acopy) _inventory (LocalVariables|GetIndex))))) false)))))))
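; BP_Pickup is a spinning world pickup that becomes a random item from PickupOptions when play begins.
; BeginPlay stores the chosen item and applies its mesh, while Tick adds a fixed yaw each frame, so spin speed depends on frame rate.
; When BP_Player enters the sphere, it creates a WBP_PickupPrompt initialized with the item and itself, then removes it when the player leaves.
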(event OnComponentBeginOverlap(Sphere)
  (params (OverlappedComponent :type Primitive%20Component%20Object%20Reference) (OtherActor :type Actor%20Object%20Reference) (OtherComp :type Primitive%20Component%20Object%20Reference) (OtherBodyIndex :type Integer) (bFromSweep :type Boolean) (SweepResult :type Hit%20Result%20Structure%20%28by%20ref%29))
  ;[1 1 1] On overlap, check if it's the player, if it is, show the pickup prompt
  (Utilities|Casting|CastToBP_Player OtherActor)
  (bind _returnvalue (UserInterface|CreateWidget "/Game/PYNK_LOOK_HERE/Blueprints/Widgets/WBP_PickupPrompt.WBP_PickupPrompt_C"))
  (bind _output_get (Variables|Default|SetPrompt _returnvalue))
  (UserInterface|Viewport|AddtoViewport _output_get 0)
  (Default|Init (Variables|Default|GetPrompt) (Variables|Default|GetPickup) self))

(event OnComponentEndOverlap(Sphere)
  (params (OverlappedComponent :type Primitive%20Component%20Object%20Reference) (OtherActor :type Actor%20Object%20Reference) (OtherComp :type Primitive%20Component%20Object%20Reference) (OtherBodyIndex :type Integer))
  ;[1 1 1] On overlap, check if it's the player, if it is, show the pickup prompt
  (Utilities|Casting|CastToBP_Player OtherActor)
  (Widget|RemovefromParent (Variables|Default|GetPrompt)))

(event EventBeginPlay
  ;[1 1 1] Makes it a random pickup
  (bind _output_get (Variables|Default|SetPickup (.OutItem (Utilities|Array|Random (Variables|Default|GetPickupOptions)))))
  (Components|StaticMesh|SetStaticMesh (Variables|Default|GetStaticMesh) (.mesh _output_get)))

(event EventTick
  (params (DeltaSeconds :type Float%20%28single-precision%29))
  ;[1 1 1] Weeeeeeeeeeeeeeeeee
  (Class|Actor|AddActorWorldRotation "0.000000,2.000000,0.000000"))

(fn ConstructionScript)